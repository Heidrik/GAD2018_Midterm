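; Saw trap actor that slides and spins a blade and hurts the third-person player character on contact.
; On BeginPlay it starts two timelines: one lerps the Saw's relative location along local X, the other drives its yaw.
; A Collision overlap casts to BP_ThirdPersonCharacter, calls its DamageFunction with a fixed amount and prints a debug string.
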(event OnComponentBeginOverlap(Collision)
  (params (OverlappedComponent :type Primitive%20Component%20Object%20Reference) (OtherActor :type Actor%20Object%20Reference) (OtherComp :type Primitive%20Component%20Object%20Reference) (OtherBodyIndex :type Integer) (bFromSweep :type Boolean) (SweepResult :type Hit%20Result%20Structure%20%28by%20ref%29))
  (bind _asbp_third_person_character (Utilities|Casting|CastToBP_ThirdPersonCharacter OtherActor))
  (Default|DamageFunction _asbp_third_person_character -25.0)
  (Development|PrintString "Hello"))

(event EventBeginPlay
  (bind _saw (Variables|Default|GetSaw))
  (Utilities|FlowControl|Sequence
    (:then_0
      (bind _move (Timeline|LeftRight Play)
        (:Update
          (Transformation|SetRelativeLocation _saw (Math|Vector|Lerp(Vector) "0, 0, 0" "-160.000000,0.000000,0.000000" _move) false false))))
    (:then_1
      (bind _newtrack_0 (Timeline|Spin Play)
        (:Update
          (Transformation|SetRelativeRotation _saw (Math|Rotator|MakeRotator 0.0 0.0 _newtrack_0) false false))))))

(event Collision|EventActorBeginOverlap
  (params (OtherActor :type Actor%20Object%20Reference)))

(fn ConstructionScript)