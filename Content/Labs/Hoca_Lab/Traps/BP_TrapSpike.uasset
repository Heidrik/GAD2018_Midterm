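; BP_TrapSpike is a spike trap that damages the third-person player character.
; When the player enters ActivisionBox, a Timeline moves the spike mesh along Z.
; A separate Box calls DamageFunction with a fixed amount on any overlapping BP_ThirdPersonCharacter and prints a debug string.
; On BeginPlay it binds to the character's trap event, which destroys the spikes, damage box and Timeline when the trap type matches.
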(event OnComponentBeginOverlap(ActivisionBox)
  (params (OverlappedComponent :type Primitive%20Component%20Object%20Reference) (OtherActor :type Actor%20Object%20Reference) (OtherComp :type Primitive%20Component%20Object%20Reference) (OtherBodyIndex :type Integer) (bFromSweep :type Boolean) (SweepResult :type Hit%20Result%20Structure%20%28by%20ref%29))
  (if (== OtherActor (Variables|Default|GetAs%20BP%20Third%20Person%20Character))
    (bind _newtrack_0 (Timeline|Timeline Play)
      (:Update
        (Transformation|SetRelativeLocation (Variables|Default|GetSM_Spikes) (Math|Vector|MakeVector 0.0 0.0 _newtrack_0) false false)))))

(event OnComponentBeginOverlap(Box)
  (params (OverlappedComponent :type Primitive%20Component%20Object%20Reference) (OtherActor :type Actor%20Object%20Reference) (OtherComp :type Primitive%20Component%20Object%20Reference) (OtherBodyIndex :type Integer) (bFromSweep :type Boolean) (SweepResult :type Hit%20Result%20Structure%20%28by%20ref%29))
  (bind _asbp_third_person_character (Utilities|Casting|CastToBP_ThirdPersonCharacter OtherActor))
  (Default|DamageFunction _asbp_third_person_character -15.0)
  (Development|PrintString "Hello"))

(event Custom|DP_Trap_Event
  (params (TrapType :type TrapType%20Enum :default "NewEnumerator0"))
  (if (Utilities|Enum|Equal(Enum) (Variables|Default|GetTrap%20Type) TrapType)
    (Components|DestroyComponent (Variables|Default|GetSM_Spikes))))

(event EventBeginPlay
  (bind _asbp_third_person_character (Utilities|Casting|CastToBP_ThirdPersonCharacter (Game|GetPlayerCharacter 0)))
  (bind _output_get (Variables|Default|SetAs%20BP%20Third%20Person%20Character _asbp_third_person_character))
  (EventDispatchers|BindEventtoDPTraps _output_get (delegate Custom|DP_Trap_Event)))

(event Collision|EventActorBeginOverlap
  (params (OtherActor :type Actor%20Object%20Reference)))

(event EventTick
  (params (DeltaSeconds :type Float%20%28single-precision%29)))

(fn ConstructionScript)